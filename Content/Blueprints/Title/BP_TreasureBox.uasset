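; BP_TreasureBox is a title-folder treasure box actor that slowly spins its SpringArm around the vertical axis.
; BeginPlay resets the speed, then each Tick raises it by a small step up to a cap and applies it as world yaw, easing the rotation in.
; The ramp and rotation are per frame without delta-time scaling, so both depend on frame rate.
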(event `self.ReceiveBeginPlay`
  (set `self.CurrentSpeed` 0.0)
  (set `self.MaxSpeed` 0.2))

(event `self.ReceiveTick`
  (params (DeltaSeconds :type "Float (single-precision)"))
  (bind _output_get (set `self.CurrentSpeed` (+ (`self.CurrentSpeed`) 0.0001)))
  (if (>= _output_get (`self.MaxSpeed`))
    (set `self.CurrentSpeed` (`self.MaxSpeed`)))
  (`SceneComponent.K2_AddWorldRotation` (`self.SpringArm`) (`KismetMathLibrary.MakeRotator` 0.0 0.0 (`self.CurrentSpeed`)) false false))

(fn `UserConstructionScript`)