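; AI controller for Spirit enemies that starts the BP_SpiritBT behavior tree on BeginPlay.
; The controller does nothing else at runtime, as its Tick, OnPossess and construction script are empty.
; An unconnected chain, which never runs, would seed BP_SpiritBB with the pawn's home location, a random nearby navigable target and an idle time before starting the same tree.
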(event `self.ReceiveBeginPlay`
  (`self.RunBehaviorTree` "/Game/Blueprints/Enemy/Spirits/BP_SpiritBT.BP_SpiritBT"))

(event `self.OnPossess`
  (params (PossessedPawn :type "Pawn Object Reference")))

(fn `UserConstructionScript`)