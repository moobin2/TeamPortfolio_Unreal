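; BP_Spirit is a spirit enemy Blueprint that reacts to pawns it sees.
; On BeginPlay it runs the parent logic, then stores the PawnSensing sight radius as its chase range and sets a fixed peace range.
; When PawnSensing sees a pawn during one specific state, it records that pawn as Instigator, switches state and prints a debug message.
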(event `self.ReceiveBeginPlay`
  (`parent.ReceiveBeginPlay`)
  (set `self.RangeInChase` (`PawnSensingComponent.SightRadius` (`self.PawnSensing`)))
  (set `self.RangeInPeace` 1000.0))

(event `self.PawnSensing.OnSeePawn`
  (params (Pawn :type "Pawn Object Reference"))
  (if (`|EnumEquality` (`self.CurrentStatePawn`) "NewEnumerator0")
    (set `self.Instigator` Pawn)
    (`self.SetState` "NewEnumerator2")
    (`KismetSystemLibrary.PrintString` "Saw Player")))

(fn `UserConstructionScript`
  (`parent.UserConstructionScript`))