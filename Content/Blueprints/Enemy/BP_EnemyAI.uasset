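; BP_EnemyAI is the enemy AI controller that starts behavior tree-driven logic when it possesses a pawn.
; On possess, it initializes the BP_EnemyBB blackboard with the pawn's location as home, a random navigable point around it as first target, and an idle time.
; It then runs BP_EnemyBT; BeginPlay, Tick and the construction script are empty.
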(event `self.OnPossess`
  (params (PossessedPawn :type "Pawn Object Reference"))
  (bind _returnvalue (`self.K2_GetActorLocation` (`self.K2_GetPawn`)))
  (`|ExecutionSequence`
    (:`then_0`
      (`self.UseBlackboard` "/Game/Blueprints/Enemy/BP_EnemyBB.BP_EnemyBB")
      (`BlackboardComponent.SetValueAsVector` (`self.Blackboard`) (`self.HomeLocKey`) _returnvalue)
      (`BlackboardComponent.SetValueAsVector` (`self.Blackboard`) (`self.TargetLocKey`) (`NavigationSystem.K2_GetRandomLocationInNavigableRadius` _returnvalue 1000.0))
      (`BlackboardComponent.SetValueAsFloat` (`self.Blackboard`) (`self.IdleTimeKey`) 4.0))
    (:`then_1`
      (`self.RunBehaviorTree` "/Game/Blueprints/Enemy/BP_EnemyBT.BP_EnemyBT"))))

(fn `UserConstructionScript`)