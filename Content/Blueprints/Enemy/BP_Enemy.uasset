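; Enemy pawn Blueprint with health and a four-state machine (peace, chase, attack, dead), scaled up on BeginPlay.
; PawnSensing moves it from peace to chase, storing the seen pawn as Instigator; damage reaching zero HP sets dead.
; SetState locks once dead, syncs the Blackboard state key and sets scale-based walk speed: faster in chase, zero in attack or dead.
; Initial peace speed is computed before the scale-up.
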(event `self.ReceiveBeginPlay`
  (set `self.CurrentHP` (`self.MaxHP`))
  (`self.SetState` "NewEnumerator0")
  (`self.SetActorScale3D` (3.0 3.0 3.0)))

(event `self.ReceiveAnyDamage`
  (params (Damage :type "Float (single-precision)") (DamageType :type "DamageType Object Reference") (InstigatedBy :type "Controller Object Reference") (DamageCauser :type "Actor Object Reference"))
  (bind _output_get (set `self.CurrentHP` (- (`self.CurrentHP`) Damage)))
  (if (> _output_get 0.0)
    (`KismetSystemLibrary.PrintString` (`KismetStringLibrary.Conv_DoubleToString` _output_get))
    (else
      (`self.SetState` "NewEnumerator3"))))

(event `self.PawnSensing.OnSeePawn`
  (params (Pawn :type "Pawn Object Reference"))
  ;[1 1 1] Player 가 감지되면 State 를 CHASE 로 한 번만 변경
  (if (`|EnumEquality` (`self.CurrentStatePawn`) "NewEnumerator0")
    (set `self.Instigator` Pawn) ; 감지된 플레이어 저장
    (`self.SetState` "NewEnumerator1")))

(fn `SetState`
  (params (NewState :type "/Game/Blueprints/Enemy/BPE_EnemyState Enum"))
  (bind _returnvalue_x (`KismetMathLibrary.BreakVector` (`self.GetActorScale3D`)))
  (bind _charactermovement (`self.CharacterMovement`))
  (bind _returnvalue (* _returnvalue_x (`self.WalkSpeed`)))
  (if (`|EnumInequality` (`self.CurrentStatePawn`) "NewEnumerator3")
    (bind _output_get (set `self.CurrentStatePawn` NewState))
    ;[1 1 1] 상태 체크용
    (`KismetSystemLibrary.PrintString` (`|GetEnumeratorNameAsString` _output_get))
    (`|ExecutionSequence`
      (:`then_0`
        ;[1 1 1] BlackBoard 의 State 값 동기화
        (`BlackboardComponent.SetValueAsEnum` (`AIBlueprintHelperLibrary.GetBlackboard` (`self.GetController`)) (`self.StateKey`) _output_get))
      (:`then_1`
        (switch `/Game/Blueprints/Enemy/BPE_EnemyState` _output_get
          (:`NewEnumerator0`
            (set `CharacterMovementComponent.MaxWalkSpeed` _returnvalue _charactermovement))
          (:`NewEnumerator1`
            (set `CharacterMovementComponent.MaxWalkSpeed` (* _returnvalue 1.2) _charactermovement))
          (:`NewEnumerator2`
            (set `CharacterMovementComponent.MaxWalkSpeed` (* _returnvalue 0.0) _charactermovement :!label _label))
          (:`NewEnumerator3`
            (goto _label)))))))

(fn `UserConstructionScript`)