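; Title camera actor that becomes the first player's view on BeginPlay and orbits around its spring arm pivot.
; Each Tick grows a per-frame yaw step up to a small cap and applies it as world rotation to the SpringArm, so the spin eases in to a steady speed.
; The motion ignores delta time, so it varies with frame rate; older rotation variants remain unconnected.
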(event `self.ReceiveBeginPlay`
  (set `self.Angle` 0.0)
  (`PlayerController.SetViewTargetWithBlend` (`GameplayStatics.GetPlayerController` 0) (`ActorComponent.GetOwner` (`self.Camera`)) 0.0 "VTBlend_Linear" 0.0 false))

(event `self.ReceiveTick`
  (params (DeltaSeconds :type "Float (single-precision)"))
  (bind _output_get (set `self.Angle` (+ (`self.Angle`) 0.0001)))
  (if (>= _output_get 0.3)
    (set `self.Angle` 0.3))
  (`SceneComponent.K2_AddWorldRotation` (`self.SpringArm`) (`KismetMathLibrary.MakeRotator` 0.0 0.0 (`self.Angle`)) false false))

(fn `UserConstructionScript`)