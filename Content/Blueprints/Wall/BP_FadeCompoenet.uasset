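; Actor component that fades its owning StaticMeshActor out and back in, toggled through ToggleHideMesh.
; At BeginPlay it caches the slot 0 base material and creates a dynamic instance of FadeMaterial.
; Hiding swaps in that instance, and Tick moves a clamped fade value at FadeRate, shaped by FadeCurve, into its "Fade" parameter.
; Once fully faded back in, Tick restores the base material.
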(event `self.ReceiveBeginPlay`
  (bind _asstatic_mesh_actor (cast `StaticMeshActor` (`self.GetOwner`)))
  (bind _output_get (set `self.ParentMesh` _asstatic_mesh_actor))
  (bind _asmaterial (cast `Material` (`PrimitiveComponent.GetMaterial` (`StaticMeshActor.StaticMeshComponent` _output_get) 0)))
  (set `self.BaseMaterial` _asmaterial)
  (bind _returnvalue (`KismetMaterialLibrary.CreateDynamicMaterialInstance` (`self.FadeMaterial`)))
  (set `self.FadeMaterialMID` _returnvalue))

(event `self.ReceiveTick`
  (params (DeltaSeconds :type "Float (single-precision)"))
  (`/Engine/EditorBlueprintResources/StandardMacros.IsValid` (`self.ParentMesh`)
    (:`Is Valid`
      (set `self.DeltaTime` DeltaSeconds)
      (if (`self.IsHidden`)
        (set `self.CurrentFade` (`KismetMathLibrary.FClamp` (- (`self.CurrentFade`) (* (`self.DeltaTime`) (`self.FadeRate`)))))
        (else
          (set `self.CurrentFade` (`KismetMathLibrary.FClamp` (+ (`self.CurrentFade`) (* (`self.DeltaTime`) (`self.FadeRate`)))))))
      (`MaterialInstanceDynamic.SetScalarParameterValue` (`self.FadeMaterialMID`) "Fade" (`CurveFloat.GetFloatValue` (`self.FadeCurve`) (`self.CurrentFade`)))
      (if (and (== (`self.CurrentFade`) 1.0) (not (`self.IsHidden`)))
        (`PrimitiveComponent.SetMaterial` (`StaticMeshActor.StaticMeshComponent` (`self.ParentMesh`)) 0 (`self.BaseMaterial`))))))

(fn `ToggleHideMesh`
  (params (Hidden :type Boolean))
  (if (!= Hidden (`self.IsHidden`))
    (bind _output_get (set `self.IsHidden` Hidden))
    (if _output_get
      (`PrimitiveComponent.SetMaterial` (`StaticMeshActor.StaticMeshComponent` (`self.ParentMesh`)) 0 (`self.FadeMaterialMID`)))))