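; Warrior character Blueprint, extending a parent character with gender-specific skins that change at milestone levels, refreshed on BeginPlay and on an L-key level-up.
; Key 3 enters the jump-attack skill state and activates JumpAttackComponent; a left click then starts the dash, or a normal attack when at peace.
; Spin and slash events spawn scaled fire particles, with a spin counter returning the state to PEACE once exhausted.
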(event `self.ReceiveBeginPlay`
  (`parent.ReceiveBeginPlay`)
  (`KismetSystemLibrary.PrintString` "warrior call")
  (`ActorComponent.Deactivate` (`self.JumpAttackComponent`))
  (if (`|EnumEquality` (`self.Gender`) "NewEnumerator0")
    (`self.SetMaleWarriorMaterials`)
    (else
      (`self.SetFemaleWarriorMaterials`))))

(event `Key|L`
  (params (Key :type "Key Structure" :default "AnyKey"))
  ;[1 1 1] LevelUp
  (:`Pressed`
    (`self.LevelUp`)
    (`KismetSystemLibrary.PrintString` "Warrior Set Material Call")
    (if (`|EnumEquality` (`self.Gender`) "NewEnumerator0")
      (`self.SetMaleWarriorMaterials`)
      (else
        (`self.SetFemaleWarriorMaterials`)))))

(event `SpinAttackEffect`
  ;[1 1 1] Spin Attack Effect Setting
  (if (> (`self.SpinCount`) 0)
    (if (== (`self.SpinCount`) 3)
      (bind _returnvalue (`GameplayStatics.SpawnEmitterAttached` "/Game/Asset/CustomEffect/P_AOE_Fire_CircleAttack_Custom.P_AOE_Fire_CircleAttack_Custom" (`self.K2_GetRootComponent`) "None" (`self.K2_GetActorLocation`) (struct) "KeepWorldPosition"))
      (`SceneComponent.SetRelativeScale3D` _returnvalue (0.5 0.5 0.5)))
    (set `self.SpinCount` (- (`self.SpinCount`) 1))
    (else
      (set `self.CurrentState` "NewEnumerator6")
      (set `self.SpinCount` 3))))

(event `self.ReceiveTick`
  (params (DeltaSeconds :type "Float (single-precision)"))
  (`parent.ReceiveTick` DeltaSeconds))

(event `Key|Three`
  (params (Key :type "Key Structure" :default "AnyKey"))
  (bind _jumpattackcomponent (`self.JumpAttackComponent`))
  ;[1 1 1] JumpAttack Component active
  (:`Pressed`
    (if (`|EnumEquality` (`self.CurrentState`) "NewEnumerator6")
      (set `self.SkillNumber` 3)
      (set `self.CurrentState` "NewEnumerator7")
      (if (`ActorComponent.IsActive` (`self.JumpAttackComponent`))
        (`ActorComponent.Deactivate` _jumpattackcomponent))
      (`ActorComponent.Activate` _jumpattackcomponent false))))

(event `SlashEffect`
  (bind _returnvalue_x (`KismetMathLibrary.BreakVector` (`self.GetActorScale3D`)))
  ;[1 1 1] Slash Attack Effect Setting
  (bind _returnvalue (`GameplayStatics.SpawnEmitterAttached` "/Game/Asset/CustomEffect/P_Combo_Finish_Fire_Custom.P_Combo_Finish_Fire_Custom" (`self.K2_GetRootComponent`) "None" (+ (`self.K2_GetActorLocation`) (* (`self.GetActorForwardVector`) (* _returnvalue_x 50.0))) (`KismetMathLibrary.ComposeRotators` (`self.K2_GetActorRotation`) (struct :`Yaw` 180.0)) "KeepWorldPosition"))
  (`SceneComponent.SetRelativeScale3D` _returnvalue (0.3 0.3 0.3)))

(event `Key|LeftMouseButton`
  (params (Key :type "Key Structure" :default "AnyKey"))
  (bind _jumpattackcomponent (`self.JumpAttackComponent`))
  ;[1 1 1] Mouse Left Click Event
  (:`Pressed`
    (switch `/Game/Blueprints/Character/BP_EState` (`self.CurrentState`)
      (:`NewEnumerator6`
        (`self.SetCharacterAttackState`))
      (:`NewEnumerator7`
        (if (== (`self.SkillNumber`) 3)
          (`/Game/Blueprints/Character/BP_JumpAttackComponent.SetDashSpeed` _jumpattackcomponent)
          (set `/Game/Blueprints/Character/BP_JumpAttackComponent.IsClick` true _jumpattackcomponent)
          (set `self.CurrentState` "NewEnumerator5"))))))

(event `self.JumpAttackComponent.OnComponentActivated`
  (params (Component :type "ActorComponent Object Reference") (bReset :type Boolean))
  ;[1 1 1] JumpAttack Skill Setting
  (`/Game/Blueprints/Character/BP_JumpAttackComponent.SetInitVariable` (`self.JumpAttackComponent`) 1.0 (`self.K2_GetActorLocation`)))

(fn `SetFemaleWarriorMaterials`
  (bind _mesh (`self.Mesh`))
  (switch `string` (`KismetStringLibrary.Conv_IntToString` (`self.Level`))
    (:`1`
      (`PrimitiveComponent.SetMaterial` _mesh 0 "/Game/Asset/LittleHerosCharacter/Metarials/M_FemaleSkin.M_FemaleSkin"))
    (:`2`
      (`PrimitiveComponent.SetMaterial` _mesh 0 "/Game/Asset/LittleHerosCharacter/Metarials/M_FemaleWarriorSkin1.M_FemaleWarriorSkin1"))
    (:`4`
      (`PrimitiveComponent.SetMaterial` _mesh 0 "/Game/Asset/LittleHerosCharacter/Metarials/M_FemaleWarriorSkin2.M_FemaleWarriorSkin2"))
    (:`7`
      (`PrimitiveComponent.SetMaterial` _mesh 0 "/Game/Asset/LittleHerosCharacter/Metarials/M_FemaleWarriorSkin3.M_FemaleWarriorSkin3"))
    (:`10`
      (`PrimitiveComponent.SetMaterial` _mesh 0 "/Game/Asset/LittleHerosCharacter/Metarials/M_FemaleWarriorSkin4.M_FemaleWarriorSkin4"))))

(fn `SetMaleWarriorMaterials`
  (bind _mesh (`self.Mesh`))
  (switch `string` (`KismetStringLibrary.Conv_IntToString` (`self.Level`))
    (:`1`
      (`PrimitiveComponent.SetMaterial` _mesh 0 "/Game/Asset/LittleHerosCharacter/Metarials/M_MaleSkin.M_MaleSkin"))
    (:`2`
      (`PrimitiveComponent.SetMaterial` _mesh 0 "/Game/Asset/LittleHerosCharacter/Metarials/M_MaleWarriorSkin1.M_MaleWarriorSkin1"))
    (:`4`
      (`PrimitiveComponent.SetMaterial` _mesh 0 "/Game/Asset/LittleHerosCharacter/Metarials/M_MaleWarriorSkin2.M_MaleWarriorSkin2"))
    (:`7`
      (`PrimitiveComponent.SetMaterial` _mesh 0 "/Game/Asset/LittleHerosCharacter/Metarials/M_MaleWarriorSkin3.M_MaleWarriorSkin3"))
    (:`10`
      (`PrimitiveComponent.SetMaterial` _mesh 0 "/Game/Asset/LittleHerosCharacter/Metarials/M_MaleWarriorSkin4.M_MaleWarriorSkin4"))))

(fn `UserConstructionScript`
  (`parent.UserConstructionScript`))