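; Base player character that drives a CurrentState machine (peace, jump, rolling, dash, attack, skill) from key input.
; In PEACE, Tick runs one of three F1–F3 movement schemes, move-facing or cursor-facing via a hit under the mouse, and times out the attack combo counter.
; Roll and dash call SlowMoveSpeed, whose deceleration logic is disconnected.
; It also provides level-up with particles, attack-state counting, and camera-shake and force keys.
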(event `self.ReceiveBeginPlay`
  (bind _returnvalue_x (`KismetMathLibrary.BreakVector` (`self.GetActorScale3D`)))
  (`KismetSystemLibrary.PrintString` "Base call")
  (`self.SetActorScale3D` (3.0 3.0 3.0))
  (set `SpringArmComponent.TargetArmLength` (* _returnvalue_x 300.0) (`self.SpringArm`))
  (set `self.CurrentState` "NewEnumerator6"))

(event `Key|SpaceBar`
  (params (Key :type "Key Structure" :default "AnyKey"))
  ;[1 1 1] 이동을 제외한 키 이벤트
  (:`Pressed`
    (`self.Jump`)
    (set `self.CurrentState` "NewEnumerator4")))

(event `self.ReceiveTick`
  (params (DeltaSeconds :type "Float (single-precision)"))
  (bind _returnvalue (`self.GetController`))
  (bind _speedinfo_peacespeed (break `/Game/Blueprints/Character/BP_SMoveSpeed` (`self.SpeedInfo`)))
  (switch `/Game/Blueprints/Character/BP_EState` (`self.CurrentState`)
    (:`NewEnumerator6`
      (`|ExecutionSequence`
        (:`then_0`
          (switch `int` (`self.MoveMethod`)
            (:`1`
              ;[1 1 1] 회전 및 정면으로 이동
              (if (or (!= (`self.GetInputAxisValue`) 0.0) (!= (`self.GetInputAxisValue`) 0.0))
                (`Controller.SetControlRotation` (`self.GetController`) (`KismetMathLibrary.MakeRotFromX` (`KismetMathLibrary.MakeVector` (`self.GetInputAxisValue`) (`self.GetInputAxisValue`))))
                (bind _output_get (set `self.MoveSpeed` _speedinfo_peacespeed))
                (`self.AddMovementInput` (`self.GetActorForwardVector`) _output_get)))
            (:`2`
              ;[1 1 1] 엔터더건전식
              (if (or (!= (`self.GetInputAxisValue`) 0.0) (!= (`self.GetInputAxisValue`) 0.0))
                (bind _output_get_2 (set `self.MoveSpeed` 0.5))
                (`self.AddMovementInput` (`KismetMathLibrary.GetForwardVector` (`KismetMathLibrary.MakeRotFromX` (`KismetMathLibrary.MakeVector` (`self.GetInputAxisValue`) (`self.GetInputAxisValue`)))) _output_get_2)
                (bind _mouseworldpos (`self.CalculateMousePos`))
                (bind _returnvalue_2 (`KismetMathLibrary.FindLookAtRotation` (`self.K2_GetActorLocation`) _mouseworldpos))
                (`self.K2_SetActorRotation` _returnvalue_2)
                (`Controller.SetControlRotation` (`self.GetController`) _returnvalue_2)))
            (:`3`
              ;[1 1 1] 마우스방향이 정면, 정면으로 기준으로 움직인다
              (if (or (!= (`self.GetInputAxisValue`) 0.0) (!= (`self.GetInputAxisValue`) 0.0))
                (bind _output_get_3 (set `self.MoveSpeed` 0.5))
                (bind _mouseworldpos_2 (`self.CalculateMousePos`))
                (bind _returnvalue_3 (`KismetMathLibrary.FindLookAtRotation` (`self.K2_GetActorLocation`) _mouseworldpos_2))
                (`self.K2_SetActorRotation` _returnvalue_3)
                (`Controller.SetControlRotation` _returnvalue _returnvalue_3)
                (`self.AddMovementInput` (`KismetMathLibrary.GreaterGreater_VectorRotator` (`self.GetActorForwardVector` _returnvalue) (`KismetMathLibrary.MakeRotFromX` (`KismetMathLibrary.MakeVector` (`self.GetInputAxisValue`) (`self.GetInputAxisValue`)))) _output_get_3)))))
        (:`then_1`
          ;[1 1 1] Attack카운트 관리
          (if (> (`self.AttackCount`) 0)
            (set `self.AttackTime` (+ (`self.AttackTime`) (`GameplayStatics.GetWorldDeltaSeconds`)))
            (if (> (`self.AttackTime`) 0.3)
              (set `self.AttackCount` 0)
              (set `self.AttackTime` 0.0))))))
    (:`NewEnumerator2`
      (`self.SlowMoveSpeed` :!label _label))
    (:`NewEnumerator5`
      (goto _label))))

(event `Key|RightMouseButton`
  (params (Key :type "Key Structure" :default "AnyKey"))
  (bind (_speedinfo_peacespeed _speedinfo_dashspeed _speedinfo_rollingspeed) (break `/Game/Blueprints/Character/BP_SMoveSpeed` (`self.SpeedInfo`)))
  ;[1 1 1] 이동을 제외한 키 이벤트
  (:`Pressed`
    (if (> (`KismetMathLibrary.VSize` (`MovementComponent.Velocity` (`self.CharacterMovement`))) 0.0)
      (set `self.CurrentState` "NewEnumerator2")
      (set `self.MoveSpeed` _speedinfo_rollingspeed))))

(event `Key|G`
  (params (Key :type "Key Structure" :default "AnyKey"))
  ;[1 1 1] 이동을 제외한 키 이벤트
  (:`Pressed`
    (`GameplayStatics.PlayWorldCameraShake` "/Game/Blueprints/Camera/BP_CameraShake.BP_CameraShake_C" (`PlayerCameraManager.GetCameraLocation` (`GameplayStatics.GetPlayerCameraManager` 0)) 0.0 500.0)))

(event `Key|F`
  (params (Key :type "Key Structure" :default "AnyKey"))
  (bind _returnvalue (`GameplayStatics.GetPlayerCharacter` 0))
  ;[1 1 1] 이동을 제외한 키 이벤트
  (:`Pressed`
    (`CharacterMovementComponent.AddForce` (`Character.CharacterMovement` _returnvalue) (`self.GetActorForwardVector` _returnvalue))))

(event `Key|One`
  (params (Key :type "Key Structure" :default "AnyKey"))
  ;[1 1 1] 이동을 제외한 키 이벤트
  (:`Pressed`
    (set `self.SkillNumber` 1)
    (set `self.CurrentState` "NewEnumerator7" :!label _label_2)))

(event `Key|Two`
  (params (Key :type "Key Structure" :default "AnyKey"))
  ;[1 1 1] 이동을 제외한 키 이벤트
  (:`Pressed`
    (set `self.SkillNumber` 2)
    (goto _label_2)))

(event `Key|Three`
  (params (Key :type "Key Structure" :default "AnyKey"))
  ;[1 1 1] 이동을 제외한 키 이벤트
  (:`Pressed`
    (set `self.SkillNumber` 3)
    (goto _label_2)))

(event `Key|Four`
  (params (Key :type "Key Structure" :default "AnyKey"))
  ;[1 1 1] 이동을 제외한 키 이벤트
  (:`Pressed`
    (set `self.SkillNumber` 4)
    (goto _label_2)))

(event `Key|F1`
  (params (Key :type "Key Structure" :default "AnyKey"))
  ;[1 1 1] 이동을 제외한 키 이벤트
  (:`Pressed`
    (set `self.MoveMethod` 1)))

(event `Key|F2`
  (params (Key :type "Key Structure" :default "AnyKey"))
  ;[1 1 1] 이동을 제외한 키 이벤트
  (:`Pressed`
    (set `self.MoveMethod` 2)))

(event `Key|F3`
  (params (Key :type "Key Structure" :default "AnyKey"))
  ;[1 1 1] 이동을 제외한 키 이벤트
  (:`Pressed`
    (set `self.MoveMethod` 3)))

(fn `CalculateMousePos`
  (returns (MouseWorldPos :type "Vector Structure"))
  (bind (_returnvalue_x _returnvalue_y _returnvalue_z) (`KismetMathLibrary.BreakVector` (`self.K2_GetActorLocation`)))
  (bind (_bblockinghit _binitialoverlap _time _location) (`GameplayStatics.BreakHitResult` (`PlayerController.GetHitResultUnderCursorByChannel` (`GameplayStatics.GetPlayerController` 0) "TraceTypeQuery1" true)))
  (return (`KismetMathLibrary.MakeVector` (.x _location) (.y _location) _returnvalue_z)))

(fn `LevelUp`
  (`KismetSystemLibrary.PrintString` "Level UP!")
  (bind _output_get (set `self.Level` (+ (`self.Level`) 1)))
  (`KismetSystemLibrary.PrintString` (`KismetStringLibrary.Conv_IntToString` _output_get))
  (bind _returnvalue (`GameplayStatics.SpawnEmitterAttached` "/Game/Asset/CustomEffect/P_levelUpCustom.P_levelUpCustom" (`self.K2_GetRootComponent`) "None" (`self.K2_GetActorLocation`) (struct) "KeepWorldPosition"))
  (`SceneComponent.SetRelativeScale3D` _returnvalue (0.2 0.2 0.2)))

(fn `SetCharacterAttackState`
  (set `self.CurrentState` "NewEnumerator3")
  (set `self.AttackCount` (+ (`self.AttackCount`) 1))
  (if (>= (`self.AttackCount`) 3)
    (set `self.AttackCount` 0)))

(fn `SlowMoveSpeed`
  (if (<= (`KismetMathLibrary.VSize` (`MovementComponent.Velocity` (`self.CharacterMovement`))) 0.0)
    _))

(fn `UserConstructionScript`)