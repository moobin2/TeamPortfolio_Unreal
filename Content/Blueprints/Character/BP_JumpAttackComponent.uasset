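; Player component for a mouse-aimed jump attack that dashes the character to a chosen ground point.
; While active, Tick rotates the player toward the cursor trace and redraws a one-frame decal, clamped to weapon-scaled Range, as TargetPos.
; Once IsClick is set, movement input drives the character forward at DashSpeed until near the target or one second passes.
; External callers handle initialization, dash speed calculation and charge/dash particle events.
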(event `self.ReceiveBeginPlay`
  (set `self.Range` 600.0))

(event `self.ReceiveTick`
  (params (DeltaSeconds :type "Float (single-precision)"))
  (bind _returnvalue (`GameplayStatics.GetPlayerCharacter` 0))
  ;[1 1 1] Look at mouse / Dash to Target
  (if (`self.IsActive`)
    (if (`self.IsClick`)
      (if (not (`self.IsArrive`))
        (`Pawn.AddMovementInput` _returnvalue (`Actor.GetActorForwardVector` _returnvalue) (`self.DashSpeed`) false) ; 타겟위치로 대쉬하자
        (set `self.Time` (+ (`self.Time`) (`GameplayStatics.GetWorldDeltaSeconds`)))
        (if (or (> (`self.Time`) 1.0) (<= (`KismetMathLibrary.VSize` (- (`self.TargetPos`) (`SceneComponent.K2_GetComponentLocation` (`Character.CapsuleComponent` _returnvalue)))) 50.0))
          (set `self.IsArrive` true)))
      (else
        (bind _mousepos (`self.RotateToMouse`)) ; 마우스 방향보고 회전
        (`self.DrawDacal` _mousepos) ; 마우스 위치에 데칼 그려라(공격범위내로)
      ))))

(event `ChargeEffect`
  (bind _returnvalue (`GameplayStatics.GetPlayerPawn` 0))
  ;[1 1 1] ChargeEffect On
  (bind _returnvalue_2 (`GameplayStatics.SpawnEmitterAttached` "/Game/Asset/CustomEffect/P_Circle_ChargeUp_Fire_Custom.P_Circle_ChargeUp_Fire_Custom" (`Actor.K2_GetRootComponent` _returnvalue) "None" (`Actor.K2_GetActorLocation` _returnvalue) (struct) "KeepWorldPosition"))
  (`SceneComponent.SetRelativeScale3D` _returnvalue_2 (0.6 0.6 0.6)))

(event `DashEffect`
  (bind _returnvalue (`GameplayStatics.GetPlayerPawn` 0))
  ;[1 1 1] DashEffect On
  (bind _returnvalue_2 (`GameplayStatics.SpawnEmitterAttached` "/Game/Asset/CustomEffect/P_Dash_Custom.P_Dash_Custom" (`Actor.K2_GetRootComponent` _returnvalue) "None" (- (`Actor.K2_GetActorLocation` _returnvalue) (* (`Actor.GetActorForwardVector` _returnvalue) 10.0)) (`Actor.K2_GetActorRotation` _returnvalue) "KeepWorldPosition"))
  (`SceneComponent.SetRelativeScale3D` _returnvalue_2 (0.3 0.3 0.3)))

(fn `DrawDacal`
  (params (MousePos :type "Vector Structure"))
  (locals (DecalPosInRange :type "Vector Structure"))
  (if (> (`KismetMathLibrary.VSize` (- MousePos (`self.StartPos`))) (`self.Range`))
    (set `local.DecalPosInRange` (+ (* (`Actor.GetActorForwardVector` (`GameplayStatics.GetPlayerController` 0)) (`self.Range`)) (`self.StartPos`)))
    (else
      (set `local.DecalPosInRange` MousePos)))
  (`GameplayStatics.SpawnDecalAtLocation` "/Game/Asset/Decal/M_MousePosDacel.M_MousePosDacel" (70.0 70.0 70.0) (- (`local.DecalPosInRange`) (0.0 0.0 100.0)) (struct :`Pitch` -90.0) (`GameplayStatics.GetWorldDeltaSeconds`))
  (set `self.TargetPos` (`local.DecalPosInRange`))
  (return))

(fn `RotateToMouse`
  (returns (MousePos :type "Vector Structure"))
  (bind (_startpos_x _startpos_y _startpos_z) (`KismetMathLibrary.BreakVector` (`self.StartPos`)))
  (bind (_bblockinghit _binitialoverlap _time _location) (`GameplayStatics.BreakHitResult` (`PlayerController.GetHitResultUnderCursorByChannel` (`GameplayStatics.GetPlayerController` 0) "TraceTypeQuery1" true)))
  (bind _returnvalue (`KismetMathLibrary.MakeVector` (.x _location) (.y _location) _startpos_z))
  (bind _returnvalue_2 (`KismetMathLibrary.FindLookAtRotation` (`self.StartPos`) _returnvalue))
  (`Actor.K2_SetActorRotation` (`self.GetOwner`) _returnvalue_2 false)
  (`Controller.SetControlRotation` (`GameplayStatics.GetPlayerController` 0) _returnvalue_2)
  (return _returnvalue))

(fn `SetDashSpeed`
  (set `self.DashSpeed` (* (/ (`KismetMathLibrary.VSize` (- (`self.TargetPos`) (`self.StartPos`))) 1.0) (`GameplayStatics.GetWorldDeltaSeconds`))))

(fn `SetInitVariable`
  (params (WeaponRange :type "Float (double-precision)") (CharacterPos :type "Vector Structure"))
  (`self.SetRange` WeaponRange)
  (set `self.StartPos` CharacterPos)
  (set `self.Time` 0.0)
  (set `self.IsClick` false)
  (set `self.IsArrive` false))

(fn `SetRange`
  (params (WeaponRange :type "Float (double-precision)"))
  (set `self.Range` (* WeaponRange (`self.Range`))))