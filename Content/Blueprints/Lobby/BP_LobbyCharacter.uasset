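; Lobby character Blueprint that hides itself on BeginPlay and keeps turning to face the first player's view target.
; Each Tick it sets yaw halfway between its current value and the look-at yaw, using a plain Lerp without angle wrapping or delta-time scaling.
; The LookAtCamera event is empty, and an instant-snap rotation node chain is left unconnected.
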(event `self.ReceiveBeginPlay`
  (`self.SetActorHiddenInGame` true))

(event `self.ReceiveTick`
  (params (DeltaSeconds :type "Float (single-precision)"))
  (bind (_returnvalue_roll _returnvalue_pitch _returnvalue_yaw) (`KismetMathLibrary.BreakRotator` (`self.K2_GetActorRotation`)))
  (bind (_returnvalue_roll_2 _returnvalue_pitch_2 _returnvalue_yaw_2) (`KismetMathLibrary.BreakRotator` (`KismetMathLibrary.FindLookAtRotation` (`self.K2_GetActorLocation`) (`self.K2_GetActorLocation` (`Controller.GetViewTarget` (`GameplayStatics.GetPlayerController` 0))))))
  (`self.K2_SetActorRotation` (`KismetMathLibrary.MakeRotator` 0.0 0.0 (`KismetMathLibrary.Lerp` _returnvalue_yaw _returnvalue_yaw_2 0.5))))

(event `LookAtCamera`)

(fn `UserConstructionScript`)