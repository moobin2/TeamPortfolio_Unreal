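; Base interactable item that a player picks up into their inventory.
; On BeginPlay it spawns a looping-style loot particle effect at its location and keeps a reference to it.
; Interaction checks the instigator for inventory space, sends its ItemInfo as a pickup message, then destroys itself and the effect.
; The construction script stamps the actor's own class into ItemInfo, preserving the other fields.
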(event `self.ReceiveBeginPlay`
  (bind _returnvalue (`GameplayStatics.SpawnEmitterAtLocation` "/Game/InfinityBladeEffects/Effects/FX_Treasure/Gold_Bag/P_DeadMans_Loot.P_DeadMans_Loot" (`self.K2_GetActorLocation`)))
  (set `self.Effect` _returnvalue))

(event `/Game/Blueprints/Interactable/BPI_Interact.Interaction`
  (params (Instigator :type "/Game/Blueprints/Character/BP_BaseCharacter Object Reference"))
  (if (`/Game/Blueprints/Character/BP_BaseCharacter.HasSpaceInInventory` Instigator)
    (message `/Game/Blueprints/Interactable/BPI_Interact.PickUp` Instigator (`self.ItemInfo`))
    (`self.K2_DestroyActor`)
    (`ActorComponent.K2_DestroyComponent` (`self.Effect`))))

(fn `UserConstructionScript`
  (bind (_iteminfo_itemtype _iteminfo_itemname _iteminfo_itemimage _iteminfo_itemclass _iteminfo_itemindex _iteminfo_itemslot _iteminfo_itemvalue) (break `/Game/Blueprints/Interactable/F_ItemInfo` (`self.ItemInfo`)))
  (`parent.UserConstructionScript`)
  (set `self.ItemInfo` (make `/Game/Blueprints/Interactable/F_ItemInfo` _iteminfo_itemtype _iteminfo_itemname _iteminfo_itemimage (`GameplayStatics.GetObjectClass` self) _iteminfo_itemindex _iteminfo_itemslot _iteminfo_itemvalue)))